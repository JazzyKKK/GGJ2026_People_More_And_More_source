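; Level spawn point that adds five characters to the group population, once, when its detect zones are triggered.
; On BeginPlay it binds to the triggered-changed events of two detect zones, which share one AND check on their Triggered values.
; When that check passes, a DoOnce finds the GGJCharacterGroupManager and calls AddPopulation at the SpawnPoint component's world location.
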(event `self.ReceiveBeginPlay`
  (add `GGJCountZone.OnTriggeredChanged` (`self.detect_zone`) (delegate `trigger`))
  (add `GGJCountZone.OnTriggeredChanged` (`self.detect_zone1`) (delegate `trigger2`)))

(event `trigger`
  (params (bTriggered :type Boolean))
  (if (and bTriggered (stale `trigger2` bTriggered)) :!label _label
    (`/Engine/EditorBlueprintResources/StandardMacros.DoOnce` false
      (:`Completed`
        (bind _returnvalue (`GameplayStatics.GetActorOfClass` "/Script/GGJ_gamedemo.GGJCharacterGroupManager"))
        (`GGJCharacterGroupManager.AddPopulation` _returnvalue 5 (`SceneComponent.K2_GetComponentLocation` (`self.SpawnPoint`)))))))

(event `trigger2`
  (params (bTriggered :type Boolean))
  (goto _label))

(fn `UserConstructionScript`)