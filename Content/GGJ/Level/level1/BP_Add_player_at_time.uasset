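; Level 1 actor that periodically grows the player's character group once its two linked triggers are active.
; It listens to both triggers' change events and, when both read as triggered, starts a looping timer a single time.
; Every four seconds the timer adds two characters through the group manager, spawning just above the group camera's current focus if that camera is valid.
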(event `self.ReceiveBeginPlay`
  (add `GGJCountZone.OnTriggeredChanged` (`self.Target`) (delegate `trigger1`))
  (add `GGJCountZone.OnTriggeredChanged` (`self.Target_0`) (delegate `trigger2`)))

(event `trigger2`
  (params (bTriggered :type Boolean))
  (if (and bTriggered (stale `trigger1` bTriggered)) :!label _label
    (`/Engine/EditorBlueprintResources/StandardMacros.DoOnce` false
      (:`Completed`
        (set `self.start gen` true)
        (`KismetSystemLibrary.K2_SetTimerDelegate` (delegate `gen`) 4.0 true)))))

(event `trigger1`
  (params (bTriggered :type Boolean))
  (goto _label))

(event `gen`
  (bind _returnvalue (`GameplayStatics.GetActorOfClass` "/Game/GGJ/Character/Blueprints/BP_CharacterGroupManager.BP_CharacterGroupManager_C"))
  (bind _returnvalue_2 (`GGJCharacterGroupManager.GetGroupCamera` _returnvalue))
  (if (`KismetSystemLibrary.IsValid` _returnvalue_2)
    (bind _returnvalue_3 (`GameplayStatics.GetActorOfClass` "/Script/GGJ_gamedemo.GGJCharacterGroupManager"))
    (`GGJCharacterGroupManager.AddPopulation` _returnvalue_3 2 (+ (`GGJGroupCameraActor.GetCurrentFocus` _returnvalue_2) (0.0 0.0 10.0)))))

(fn `UserConstructionScript`)