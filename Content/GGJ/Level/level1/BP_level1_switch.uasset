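; Level 1 controller Blueprint that handles background music and the exit to the Demonstration2 level through three bound triggers.
; BeginPlay fades in the first track, and Trigger2 and Trigger3 share an AND check that crossfades once to a second track.
; Trigger1Leave fires once, and only if the second track's component is valid does it fade that music out and open the next level after a matching delay.
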(event `self.ReceiveBeginPlay`
  (add `GGJCountZone.OnTriggeredChanged` (`self.trigger1_leave`) (delegate `change level`))
  (add `GGJCountZone.OnTriggeredChanged` (`self.trigger2`) (delegate `Trigger_event2`))
  (add `GGJCountZone.OnTriggeredChanged` (`self.trigger3`) (delegate `Trigger_event`))
  (bind _returnvalue (`GameplayStatics.SpawnSound2D` "/Game/GGJ/Level/level1/Music/MS_Matt_Christensen_John_Reeves_-_I_Wonder__Stars_Version_.MS_Matt_Christensen_John_Reeves_-_I_Wonder__Stars_Version_" 0.6 1.0 0.0 null false false))
  (bind _output_get (set `self.BGM_AudioComponent1` _returnvalue))
  (`AudioComponent.FadeIn` _output_get 5.0 1.0 0.0 "SCurve"))

(event `Trigger_event2`
  (params (bTriggered :type Boolean))
  (if (and bTriggered (stale `Trigger_event` bTriggered)) :!label _label
    (`/Engine/EditorBlueprintResources/StandardMacros.DoOnce` false
      (:`Completed`
        (`AudioComponent.FadeOut` (`self.BGM_AudioComponent1`) 3.0 0.0 "Linear")
        (bind _returnvalue (`GameplayStatics.SpawnSound2D` "/Game/GGJ/Level/level1/Music/MS_Matt_Christensen_-_It_s_a_Jungle__Next_Door_.MS_Matt_Christensen_-_It_s_a_Jungle__Next_Door_" 0.6 1.0 0.0 null false false))
        (bind _output_get (set `self.BGM_AudioComponent2` _returnvalue))
        (`AudioComponent.FadeIn` _output_get 3.0 1.0 0.0 "Linear")))))

(event `change level`
  (params (bTriggered :type Boolean))
  (bind _bgm_audiocomponent2 (`self.BGM_AudioComponent2`))
  (if bTriggered
    (`/Engine/EditorBlueprintResources/StandardMacros.DoOnce` false
      (:`Completed`
        (if (`KismetSystemLibrary.IsValid` _bgm_audiocomponent2)
          (`AudioComponent.FadeOut` _bgm_audiocomponent2 3.0 0.0 "Linear")
          (`KismetSystemLibrary.Delay` 3.0)
          (`GameplayStatics.OpenLevelBySoftObjectPtr` "/Game/GGJ/Level/level2/Demonstration2.Demonstration2"))))))

(event `Trigger_event`
  (params (bTriggered :type Boolean))
  (goto _label))

(fn `UserConstructionScript`)