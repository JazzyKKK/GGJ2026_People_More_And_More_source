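; Level 1 background music controller that moves from an opening track to a second one based on two level triggers.
; On BeginPlay it spawns and fades in "I Wonder (Stars Version)" and binds to both triggers' change events.
; Both events share one check that, once both triggers read as triggered, runs a DoOnce crossfade to "It's a Jungle (Next Door)".
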(event `self.ReceiveBeginPlay`
  (bind _returnvalue (`GameplayStatics.SpawnSound2D` "/Game/GGJ/Asset/Music/BGM/MS_Matt_Christensen_John_Reeves_-_I_Wonder__Stars_Version_.MS_Matt_Christensen_John_Reeves_-_I_Wonder__Stars_Version_" 0.6 1.0 0.0 null false false))
  (bind _output_get (set `self.BGM_AudioComponent1` _returnvalue))
  (`AudioComponent.FadeIn` _output_get 5.0 1.0 0.0 "SCurve")
  (add `GGJCountZone.OnTriggeredChanged` (`self.trigger1`) (delegate `Trigger_event`))
  (add `GGJCountZone.OnTriggeredChanged` (`self.trigger2`) (delegate `Trigger_event2`)))

(event `Trigger_event2`
  (params (bTriggered :type Boolean))
  (if (and bTriggered (stale `Trigger_event` bTriggered)) :!label _label
    (`/Engine/EditorBlueprintResources/StandardMacros.DoOnce` false
      (:`Completed`
        (`AudioComponent.FadeOut` (`self.BGM_AudioComponent1`) 3.0 0.0 "Linear")
        (bind _returnvalue (`GameplayStatics.SpawnSound2D` "/Game/GGJ/Asset/Music/BGM/MS_Matt_Christensen_-_It_s_a_Jungle__Next_Door_.MS_Matt_Christensen_-_It_s_a_Jungle__Next_Door_" 0.6 1.0 0.0 null false false))
        (bind _output_get (set `self.BGM_AudioComponent2` _returnvalue))
        (`AudioComponent.FadeIn` _output_get 3.0 1.0 0.0 "Linear")))))

(event `Trigger_event`
  (params (bTriggered :type Boolean))
  (goto _label))

(fn `UserConstructionScript`)