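; BP_LevelCountdown runs a level countdown that fails the player if the finish trigger is not active when time runs out.
; On BeginPlay it binds to the countdown-finished event and to TriggerFinish, whose triggered state is stored in Playerfinish and pauses the countdown when true.
; On expiry without a finish, it shows the WB_End widget, waits briefly, then resets the current level.
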(event `self.ReceiveBeginPlay`
  (add `self.OnCountdownFinished` (delegate `OnCountdownFinished_事件`))
  (add `GGJCountZone.OnTriggeredChanged` (`self.trigger_finish`) (delegate `自定义事件`)))

(event `自定义事件`
  (params (bTriggered :type Boolean))
  (bind _output_get (set `self.Playerfinish` bTriggered))
  (if _output_get
    (`self.PauseCountdown`)))

(event `OnCountdownFinished_事件`
  (if (not (`self.Playerfinish`))
    (bind _returnvalue (`|CreateWidget` "/Game/GGJ/UI/WB_End.WB_End_C" (`GameplayStatics.GetPlayerController` 0)))
    (`UserWidget.AddToViewport` _returnvalue 0)
    (`KismetSystemLibrary.Delay` 2.0)
    (`self.ResetCurrentLevel`)))

(fn `UserConstructionScript`)