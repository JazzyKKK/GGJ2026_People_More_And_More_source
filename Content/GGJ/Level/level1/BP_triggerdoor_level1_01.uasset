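; Level 1 trigger door actor that opens in response to two referenced count zones and starts the level countdown.
; Both zones' triggered-change events share one check on the triggered state.
; When it passes, a timeline swings the pivot to -90 degrees yaw, with a FlipFlop on finish alternating reverse and replay to keep it cycling.
; A DoOnce starts BP_Level_1_Countdown, found by class, on the first pass.
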(event `self.ReceiveBeginPlay`
  (add `GGJCountZone.OnTriggeredChanged` (`self.CountZoneRef1`) (delegate `HandleCountZoneTriggered`))
  (add `GGJCountZone.OnTriggeredChanged` (`self.CountZoneRef2`) (delegate `HandleCountZoneTriggered2`)))

(event `HandleCountZoneTriggered2`
  (params (bTriggered :type Boolean))
  (if (and bTriggered (stale `HandleCountZoneTriggered` bTriggered)) :!label _label
    (`|ExecutionSequence`
      (:`then_0`
        (bind (_direction `_新建轨道_0`) (`Timeline|dooranime` :!label _label_2)
          (:`Update`
            (`SceneComponent.K2_SetRelativeRotation` (`self.povit`) (`KismetMathLibrary.RLerp` (struct) (struct :`Pitch` -90.0) `_新建轨道_0`) false false))
          (:`Finished`
            (`/Engine/EditorBlueprintResources/StandardMacros.FlipFlop`
              (:`A`
                (goto _label_2 :!via `Reverse`))
              (:`B`
                (goto _label_2 :!via `PlayFromStart`))))))
      (:`then_1`
        (`/Engine/EditorBlueprintResources/StandardMacros.DoOnce` false
          (:`Completed`
            (bind _returnvalue (`GameplayStatics.GetActorOfClass` "/Game/GGJ/Level/level1/BP_Level_1_Countdown.BP_Level_1_Countdown_C"))
            (`GGJLevelCountdownActor.StartCountdown` _returnvalue -1.0)))))))

(event `HandleCountZoneTriggered`
  (params (bTriggered :type Boolean))
  (goto _label))

(fn `UserConstructionScript`)