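; Level 2 switch that completes the level when its two triggers are active, then loads L_PhysicalCharacterLab.
; On BeginPlay it binds both triggers' change events and caches the level's BP_Leve2lCountdown actor.
; Both handlers share one AND check, which on success pauses the countdown and opens the next level after a short delay.
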(event `self.ReceiveBeginPlay`
  (add `GGJCountZone.OnTriggeredChanged` (`self.trigger1`) (delegate `trigger_zone1`))
  (add `GGJCountZone.OnTriggeredChanged` (`self.trigger2`) (delegate `trigger_zone2`))
  (bind _returnvalue (`GameplayStatics.GetActorOfClass` "/Game/GGJ/Level/level2/BP_Leve2lCountdown.BP_Leve2lCountdown_C"))
  (set `self.Counter Comp` _returnvalue))

(event `trigger_zone1`
  (params (bTriggered :type Boolean))
  (if (and bTriggered (stale `trigger_zone2` bTriggered)) :!label _label
    (`GGJLevelCountdownActor.PauseCountdown` (`self.Counter Comp`))
    (`KismetSystemLibrary.Delay` 2.0)
    (`GameplayStatics.OpenLevelBySoftObjectPtr` "/Game/GGJ/Character/Maps/L_PhysicalCharacterLab.L_PhysicalCharacterLab")))

(event `trigger_zone2`
  (params (bTriggered :type Boolean))
  (goto _label))

(fn `UserConstructionScript`)