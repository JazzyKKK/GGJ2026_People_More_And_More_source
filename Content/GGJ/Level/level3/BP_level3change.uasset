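; BP_level3change handles music and the exit transition for level 3.
; On BeginPlay it spawns and fades in a 2D jungle music track and binds to a trigger zone's change event.
; When the trigger changes, it pauses the BP_level3Count countdown, fades the music out, waits briefly and opens L_PhysicalCharacterLab.
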(event `self.ReceiveBeginPlay`
  (bind _returnvalue (`GameplayStatics.SpawnSound2D` "/Game/GGJ/Asset/Music/BGM/MS_Matt_Christensen_-_It_s_a_Jungle__Next_Door_.MS_Matt_Christensen_-_It_s_a_Jungle__Next_Door_" 1.0 1.0 0.0 null))
  (bind _output_get (set `self.Sound` _returnvalue))
  (`AudioComponent.FadeIn` _output_get 1.0 1.0 0.0 "Linear")
  (add `GGJCountZone.OnTriggeredChanged` (`self.triggerzone`) (delegate `changeLevel`)))

(event `changeLevel`
  (params (bTriggered :type Boolean))
  (bind _returnvalue (`GameplayStatics.GetActorOfClass` "/Game/GGJ/Level/level3/BP_level3Count.BP_level3Count_C"))
  (`GGJLevelCountdownActor.PauseCountdown` _returnvalue)
  (`AudioComponent.FadeOut` (`self.Sound`) 0.5 0.0 "Linear")
  (`KismetSystemLibrary.Delay` 1.0)
  (`GameplayStatics.OpenLevelBySoftObjectPtr` "/Game/GGJ/Character/Maps/L_PhysicalCharacterLab.L_PhysicalCharacterLab"))

(fn `UserConstructionScript`)